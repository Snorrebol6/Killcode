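; Enemy character that turns to face and shoots the player's BP_Killcode_character when PawnSensing sees it.
; Each attack spawns a BP_SCSProjectile at SpawnLocation and applies damage directly to the player at once, without waiting for a projectile hit.
; A CanAttack flag with a short Delay limits the fire rate, while the facing snaps on every sighting.
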(event `self.PawnSensing.OnSeePawn`
  (params (Pawn :type "Pawn Object Reference"))
  (bind _asbp_killcode_character (cast `/Game/MP_Blueprints/BP_Killcode_character` Pawn))
  (`self.K2_SetActorRotation` (`KismetMathLibrary.FindRelativeLookAtRotation` (`KismetMathLibrary.Conv_VectorToTransform` (`self.K2_GetActorLocation`)) (`self.K2_GetActorLocation` _asbp_killcode_character)))
  (if (`self.CanAttack`)
    (`|SpawnActorFromClass` "/Game/MP_Blueprints/BP_SCSProjectile.BP_SCSProjectile_C" (`SceneComponent.K2_GetComponentToWorld` (`self.SpawnLocation`)) "Undefined" "MultiplyWithRoot" null null)
    (`GameplayStatics.ApplyDamage` _asbp_killcode_character 1.0)
    (set `self.CanAttack` false)
    (`KismetSystemLibrary.Delay` 0.5)
    (set `self.CanAttack` true)))

(fn `UserConstructionScript`)